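; BP_AttachBox_MC is an interactive box actor that attaches to the player character and glides toward its Scene component.
; DoAttach attaches to that component keeping world location and disables Cube collision.
; A Timeline then steps it along a recomputed direction, scaled by the TimeSpeed track, while at least 10 units away.
; DoInteraction only prints a debug string, and the Tick movement is switched off by a false condition.
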(event `/Game/BP_Class/BP_Interface_Intrection_MC.DoInteraction`
  (`KismetSystemLibrary.PrintString` "interactive"))

(event `/Game/BP_Class/BP_Interface_Intrection_MC.DoAttach`
  ; Player > Scene Comp
  (bind _asbp_third_person_character (cast `/Game/ThirdPerson/Blueprints/BP_ThirdPersonCharacter` (`GameplayStatics.GetPlayerPawn` 0)))
  (bind _scene (`/Game/ThirdPerson/Blueprints/BP_ThirdPersonCharacter.Scene` _asbp_third_person_character))
  (set `self.destLoc` (`SceneComponent.K2_GetComponentLocation` _scene))
  (set `self.dir` (`KismetMathLibrary.Normal` (- (`self.destLoc`) (`self.K2_GetActorLocation`))))
  (`self.K2_AttachToComponent` _scene "None" "KeepWorld" "KeepRelative" "KeepRelative")
  (`PrimitiveComponent.SetCollisionEnabled` (`self.Cube`) "NoCollision")
  (bind (_direction _timespeed) (`Timeline|Timeline`)
    (:`Update`
      (bind _asbp_third_person_character_2 (cast `/Game/ThirdPerson/Blueprints/BP_ThirdPersonCharacter` (`GameplayStatics.GetPlayerPawn` 0)))
      (bind _returnvalue (- (`SceneComponent.K2_GetComponentLocation` (`/Game/ThirdPerson/Blueprints/BP_ThirdPersonCharacter.Scene` _asbp_third_person_character_2)) (`self.K2_GetActorLocation`)))
      (set `self.dir` (`KismetMathLibrary.Normal` _returnvalue))
      ; P=p0 + vt
      (if (>= (`KismetMathLibrary.VSize` _returnvalue) 10.0)
        (`self.K2_SetActorLocation` (+ (`self.K2_GetActorLocation`) (* (`self.dir`) _timespeed))) ; P (바뀐 위치)
      ))))

(event `self.ReceiveTick`
  (params (DeltaSeconds :type "Float (single-precision)"))
  (if (and false (>= (`KismetMathLibrary.VSize` (- (`self.destLoc`) (`self.K2_GetActorLocation`))) 0.0))
    (`self.K2_SetActorLocation` (+ (`self.K2_GetActorLocation`) (* (`self.dir`) (* DeltaSeconds 50.0))))))

(fn `UserConstructionScript`)