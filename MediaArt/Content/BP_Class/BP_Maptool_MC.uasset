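; Map tool actor that builds a 3D grid of static mesh cubes in its construction script and can rotate itself smoothly.
; Nested loops over GridX, GridY and GridZ add the meshes floor by floor, offset from CubeLoc by GridSize.
; SmoothRot, gated by IsRot, adds DeltaRotZ to yaw through a timeline-driven quaternion slerp.
; Its timed Tick trigger is disconnected, as are several older grid-building experiments.
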(event `self.ReceiveTick`
  (params (DeltaSeconds :type "Float (single-precision)")))

(event `SmoothRot`
  (bind (_returnvalue_roll _returnvalue_pitch _returnvalue_yaw) (`KismetMathLibrary.BreakRotator` (`self.K2_GetActorRotation`)))
  (if (`self.isRot`)
    (set `self.curRot` (`self.K2_GetActorRotation`))
    (set `self.targetRot` (`KismetMathLibrary.MakeRotator` _returnvalue_roll _returnvalue_pitch (+ _returnvalue_yaw (`self.deltaRotZ`))))
    (set `self.isRot` false)
    (bind (_direction _newtrack_0) (`Timeline|rot` :!via `PlayFromStart`)
      (:`Update`
        (`self.K2_SetActorRotation` (`KismetMathLibrary.Quat_Rotator` (`KismetMathLibrary.Quat_Slerp` (`KismetMathLibrary.Conv_RotatorToQuaternion` (`self.curRot`)) (`KismetMathLibrary.Conv_RotatorToQuaternion` (`self.targetRot`)) _newtrack_0)))))))

(fn `UserConstructionScript`
  (locals (singleActorSize :type "Vector Structure"))
  (bind _gridsize (`self.gridSize`))
  (bind _gridx (`self.gridX`))
  (for _index (range (`self.gridZ`))
    (for _index_2 (range (* (`self.gridX`) (`self.gridY`)))
      (`AddComponent|NODE_AddStaticMeshComponent-6` :`RelativeTransform` (`KismetMathLibrary.MakeTransform` (+ (`self.cubeLoc`) (`KismetMathLibrary.MakeVector` (* (mod _index_2 _gridx) _gridsize) (* (/ _index_2 _gridx) _gridsize) (* _index _gridsize))))))))