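; BP_BeginCalc_MC is a game timer that counts up to GameoverTime.
; DoInteraction creates and shows the UI_Timer_MC widget, while Tick accumulates CurTime until IsPrint is set.
; The UITextUpdate event runs UITextUpdateFunc, which writes minutes and seconds to the widget or, at the limit, shows "Time is Over", freezes the count and calls StopMovement on the ThirdPersonCharacter.
; Tick never triggers that update, and leftover debug chains are unreachable.
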(event `self.ReceiveTick`
  (params (DeltaSeconds :type "Float (single-precision)"))
  ; Timer를 만들자!
  (if (not (`self.isPrint`))
    (set `self.curTime` (+ DeltaSeconds (`self.curTime`))) ; set
  ))

(event `/Game/BP_Class/BP_Interface_Intrection_MC.DoInteraction`
  (bind _returnvalue (`|CreateWidget` "/Game/BP_Class/UI_Timer_MC.UI_Timer_MC_C" (`GameplayStatics.GetPlayerController` 0)))
  (bind _output_get (set `self.uiTimerObj` _returnvalue))
  (`UserWidget.AddToViewport` _output_get 0)
  (set `/Game/BP_Class/UI_Timer_MC.uiTimeText` "Test" _output_get))

(event `self.ReceiveActorBeginOverlap`
  (params (OtherActor :type "Actor Object Reference")))

(event `UITextUpdate`
  (`self.UITextUpdateFunc`))

(fn `UITextUpdateFunc`
  (bind _curtime (`self.curTime`))
  (if (>= (`self.curTime`) (`self.gameoverTime`))
    (set `/Game/BP_Class/UI_Timer_MC.uiTimeText` "Time is Over" (`self.uiTimerObj`))
    ; PlayerPawn이 ThirdPersonCharacter가 맞다면
    ; StopMovement를 실행해라(호출해라)
    (set `self.isPrint` true)
    (bind _asbp_third_person_character (cast `/Game/ThirdPerson/Blueprints/BP_ThirdPersonCharacter` (`GameplayStatics.GetPlayerPawn` 0)))
    (`/Game/ThirdPerson/Blueprints/BP_ThirdPersonCharacter.StopMovement` _asbp_third_person_character)
    (else
      (set `/Game/BP_Class/UI_Timer_MC.uiTimeText` (`|FormatText` "{min} : {sec}" (`KismetTextLibrary.Conv_DoubleToText` (/ _curtime 60.0) "ToZero" false true 2 2 0 0) (`KismetTextLibrary.Conv_DoubleToText` (mod _curtime 60.0) "HalfToEven" false true 2 2 0 0)) (`self.uiTimerObj`)))))

(fn `UserConstructionScript`)