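; BP_Circle_MC is an actor that procedurally arranges static mesh components in a flat ring around its origin.
; The construction script divides a full circle by Piece, then uses cosine and sine to get a direction for each index.
; Each mesh is placed at that direction scaled by Dist and rotated so its X axis points outward.
; The event graph contains only disabled placeholder events, so it adds no runtime logic.
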(fn `UserConstructionScript`
  (set `self.theta` (/ (* (`KismetMathLibrary.GetPI`) 2.0) (`KismetMathLibrary.Conv_IntToDouble` (`self.piece`))))
  (for _index (range (`self.piece`))
    (bind _returnvalue (* (`KismetMathLibrary.Conv_IntToDouble` _index) (`self.theta`)))
    (bind _returnvalue_2 (`KismetMathLibrary.MakeVector` (`KismetMathLibrary.Cos` _returnvalue) (`KismetMathLibrary.Sin` _returnvalue)))
    (`AddComponent|NODE_AddStaticMeshComponent-0` :`RelativeTransform` (`KismetMathLibrary.MakeTransform` (* _returnvalue_2 (`self.dist`)) (`KismetMathLibrary.MakeRotFromX` _returnvalue_2)))))