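; BP_Array_MC is an array-practice Blueprint that totals its Score array at BeginPlay.
; A for-each loop adds each element to Number and prints the running total on screen.
; Disconnected experiments remain in the graph: an array length check, a GetAllActorsOfClass loop setting light intensities with a DirectionalLight cast, and an empty actor loop, none of which run.
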(event `self.ReceiveBeginPlay`
  ; 총합
  (for _array_element (`self.score`)
    (bind _output_get (set `self.number` (+ _array_element (`self.number`))))
    (`KismetSystemLibrary.PrintString` (`KismetStringLibrary.Conv_IntToString` _output_get) true true (struct :`G` 0.66 :`B` 1.0 :`A` 1.0) 10.0)))

(fn `UserConstructionScript`)