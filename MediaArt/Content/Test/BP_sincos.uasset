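; BP_sincos is a test Blueprint that arranges static mesh components in a ring around its origin.
; Its construction script divides a full turn by Count to get an angle step, then adds one component per index.
; Cosine and sine of each angle give a direction in the XY plane, which is scaled by Dist for location.
; MakeRotFromX turns each component to face outward along that direction.
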(fn `UserConstructionScript`
  (bind _theta (`self.theta`))
  (bind _count (`self.count`))
  (set `self.theta` (/ (* (`KismetMathLibrary.GetPI`) 2.0) (`KismetMathLibrary.Conv_IntToDouble` _count)))
  (for _index (range _count)
    (bind _returnvalue (`KismetMathLibrary.Conv_IntToDouble` _index))
    (bind _returnvalue_2 (`KismetMathLibrary.MakeVector` (`KismetMathLibrary.Cos` (* _theta _returnvalue)) (`KismetMathLibrary.Sin` (* _theta _returnvalue))))
    (`AddComponent|NODE_AddStaticMeshComponent-0` :`RelativeTransform` (`KismetMathLibrary.MakeTransform` (* _returnvalue_2 (`self.dist`)) (`KismetMathLibrary.MakeRotFromX` _returnvalue_2)))))