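; BP_Ciorcle is a test Blueprint that procedurally lays out a ring of static mesh components around the actor.
; The construction script loops over the Piece count, using cosine and sine of each index's fraction of a full turn to place a mesh on a fixed-radius circle in the XY plane.
; Each mesh's X axis points radially outward through MakeRotFromX, and the event graph holds no active logic.
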(fn `UserConstructionScript`
  (bind _piece (`self.piece`))
  (for _index (range _piece)
    (bind _returnvalue (* (/ _index _piece) (* (`KismetMathLibrary.GetPI`) 2.0)))
    (bind _returnvalue_2 (`KismetMathLibrary.MakeVector` (`KismetMathLibrary.Cos` _returnvalue) (`KismetMathLibrary.Sin` _returnvalue)))
    (`AddComponent|NODE_AddStaticMeshComponent-0` :`RelativeTransform` (`KismetMathLibrary.MakeTransform` (* _returnvalue_2 100.0) (`KismetMathLibrary.MakeRotFromX` _returnvalue_2)))))